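; Rhythm shooter game manager that owns the game, countdown and pause HUDs and runs the beat-driven target flow.
; StartCountdown leads into StartGame, which starts RhythmBeatManager and enables player shooting, while Escape toggles pausing of both.
; Each beat increments a counter used as a DT_Beatmap_Ordirehv row name, spawning BP_RhythmTarget at hardcoded lane positions.
; Hit results update score, combo and health stored on GameHUD, with game over only printed.
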(event `self.ReceiveBeginPlay`
  (bind _returnvalue (`|CreateWidget` "/Game/BeatShot/UI/GameHUD.GameHUD_C"))
  (`UserWidget.AddToViewport` _returnvalue 0)
  (bind _output_get (set `self.GameHUD` _returnvalue))
  (`/Game/BeatShot/UI/GameHUD.HideGameHUD` _output_get)
  (bind _returnvalue_2 (`|CreateWidget` "/Game/BeatShot/UI/CountdownHUD.CountdownHUD_C"))
  (`UserWidget.AddToViewport` _returnvalue_2 0)
  (bind _output_get_2 (set `self.CountdownHUD` _returnvalue_2))
  (`/Game/BeatShot/UI/CountdownHUD.HideCountdown` _output_get_2)
  (bind _returnvalue_3 (`|CreateWidget` "/Game/BeatShot/UI/PauseMenuHUD.PauseMenuHUD_C"))
  (`UserWidget.AddToViewport` _returnvalue_3 0)
  (bind _output_get_3 (set `self.PauseMenuHUD` _returnvalue_3))
  (`/Game/BeatShot/UI/PauseMenuHUD.HidePauseMenu` _output_get_3)
  (bind _asbp_shooter_character (cast `/Game/Variant_Shooter/Blueprints/BP_ShooterCharacter` (`GameplayStatics.GetPlayerCharacter` 0)))
  (set `self.Player` _asbp_shooter_character)
  (add `RhythmBeatManager.OnBeat` (`self.RhythmBeatManager`) (delegate `OnBeatReceived`)))

(event `EnhancedInput|/Game/Input/Actions/IA_Escape`
  (params (ActionValue :type Boolean) (ElapsedSeconds :type "Float (double-precision)") (TriggeredSeconds :type "Float (double-precision)") (InputAction :type "InputAction Object Reference" :default "/Game/Input/Actions/IA_Escape.IA_Escape"))
  (bind _pausemenuhud (`self.PauseMenuHUD`))
  (bind _gamehud (`self.GameHUD`))
  (:`Triggered`
    (if (`self.PauseMenuActive`)
      (`/Game/BeatShot/UI/PauseMenuHUD.HidePauseMenu` _pausemenuhud)
      (`/Game/BeatShot/UI/GameHUD.ShowGameHUD` _gamehud)
      (`self.ResumeGame`)
      (set `self.PauseMenuActive` false)
      (else
        (`/Game/BeatShot/UI/PauseMenuHUD.ShowPauseMenu` _pausemenuhud)
        (`/Game/BeatShot/UI/GameHUD.HideGameHUD` _gamehud)
        (`self.FreezeGame`)
        (set `self.PauseMenuActive` true)))))

(event `OnBeatReceived`
  (bind _result (`/Engine/EditorBlueprintResources/StandardMacros.IncrementInt` (`self.CurrentBeat`))
    (:`  `
      (set `self.CurrentBeat` _result)
      (bind _returnvalue (`|GetDataTableRow` "/Game/BeatShot/DataTables/DT_Beatmap_Ordirehv.DT_Beatmap_Ordirehv" (`KismetStringLibrary.Conv_StringToName` (`KismetStringLibrary.Conv_IntToString` (`self.CurrentBeat`))))
        (:`then`
          (bind (_beatnumber _lane) (break `/Game/BeatShot/Blueprints/S_BeatmapNote` _returnvalue))
          (`KismetSystemLibrary.PrintString` (`KismetStringLibrary.Conv_IntToString` _beatnumber))
          (bind _spawntransform (`self.GetLaneSpawnTransform` _lane))
          (`|SpawnActorFromClass` "/Game/BeatShot/Blueprints/BP_RhythmTarget.BP_RhythmTarget_C" _spawntransform "Undefined" "MultiplyWithRoot" null null))))))

(event `StartCountdown`
  (bind _countdownhud (`self.CountdownHUD`))
  (bind _countdowntext (`/Game/BeatShot/UI/CountdownHUD.CountdownText` _countdownhud))
  (`/Game/BeatShot/UI/CountdownHUD.ShowCountdown` _countdownhud)
  (`TextBlock.SetText` _countdowntext "3")
  (`KismetSystemLibrary.Delay` 1.0)
  (`TextBlock.SetText` _countdowntext "2")
  (`KismetSystemLibrary.Delay` 1.0)
  (`TextBlock.SetText` _countdowntext "1")
  (`KismetSystemLibrary.Delay` 1.0)
  (`TextBlock.SetText` _countdowntext "Start!")
  (`KismetSystemLibrary.Delay` 0.5)
  (`/Game/BeatShot/UI/CountdownHUD.HideCountdown` (`self.CountdownHUD`))
  (`self.StartGame`))

(fn `FreezeGame`
  (`RhythmBeatManager.PauseBeat` (`self.RhythmBeatManager`))
  (set `/Game/Variant_Shooter/Blueprints/BP_ShooterCharacter.CanShoot` false (`self.Player`)))

(fn `GetLaneSpawnTransform`
  (params (Lane :type Integer))
  (returns (SpawnTransform :type "Transform Structure"))
  (switch `int` Lane
    (:`0`
      (return (`KismetMathLibrary.MakeTransform` (1450.0 980.0 100.0))))
    (:`1`
      (return (`KismetMathLibrary.MakeTransform` (1450.0 1120.0 100.0))))
    (:`2`
      (return (`KismetMathLibrary.MakeTransform` (1450.0 1260.0 100.0))))
    (:`3`
      (return (`KismetMathLibrary.MakeTransform` (1450.0 1400.0 100.0))))))

(fn `ResumeGame`
  (`RhythmBeatManager.ResumeBeat` (`self.RhythmBeatManager`))
  (set `/Game/Variant_Shooter/Blueprints/BP_ShooterCharacter.CanShoot` true (`self.Player`)))

(fn `StartGame`
  (`/Game/BeatShot/UI/GameHUD.ShowGameHUD` (`self.GameHUD`))
  (`KismetSystemLibrary.PrintString` "Game Started")
  (`RhythmBeatManager.StartBeat` (`self.RhythmBeatManager`))
  (set `/Game/Variant_Shooter/Blueprints/BP_ShooterCharacter.CanShoot` true (`self.Player`)))

(fn `UpdateCombo`
  (params (HitResult :type String))
  (bind _gamehud (`self.GameHUD`))
  (bind _gamehud_2 (`self.GameHUD`))
  (switch `string` HitResult
    (:`Perfect`
      (bind _result (`/Engine/EditorBlueprintResources/StandardMacros.IncrementInt` (`/Game/BeatShot/UI/GameHUD.Combo` _gamehud))
        (:`  `
          (set `/Game/BeatShot/UI/GameHUD.Combo` _result _gamehud))))
    (:`Great`
      (bind _result_2 (`/Engine/EditorBlueprintResources/StandardMacros.IncrementInt` (`/Game/BeatShot/UI/GameHUD.Combo` _gamehud_2))
        (:`  `
          (set `/Game/BeatShot/UI/GameHUD.Combo` _result_2 _gamehud_2))))
    (:`Good`
      (set `/Game/BeatShot/UI/GameHUD.Combo` 0 (`self.GameHUD`)))
    (:`Bad`
      (set `/Game/BeatShot/UI/GameHUD.Combo` 0 (`self.GameHUD`)))
    (:`Miss`
      (set `/Game/BeatShot/UI/GameHUD.Combo` 0 (`self.GameHUD`)))))

(fn `UpdateHealth`
  (params (HitResult :type String))
  (bind _gamehud (`self.GameHUD`))
  (bind _gamehud_2 (`self.GameHUD`))
  (switch `string` HitResult
    (:`Miss`
      (set `/Game/BeatShot/UI/GameHUD.PlayerHealth` (- (`/Game/BeatShot/UI/GameHUD.PlayerHealth` _gamehud) 0.2) _gamehud)
      (if (<= (`/Game/BeatShot/UI/GameHUD.PlayerHealth` (`self.GameHUD`)) 0.0)
        (`KismetSystemLibrary.PrintString` "Game Over")))
    (:`Bad`
      (set `/Game/BeatShot/UI/GameHUD.PlayerHealth` (- (`/Game/BeatShot/UI/GameHUD.PlayerHealth` _gamehud_2) 0.1) _gamehud_2)
      (if (<= (`/Game/BeatShot/UI/GameHUD.PlayerHealth` (`self.GameHUD`)) 0.0)
        (`KismetSystemLibrary.PrintString` "Game Over")))))

(fn `UpdateScore`
  (params (HitResult :type String))
  (bind _gamehud (`self.GameHUD`))
  (bind _gamehud_2 (`self.GameHUD`))
  (bind _gamehud_3 (`self.GameHUD`))
  (bind _gamehud_4 (`self.GameHUD`))
  (bind _gamehud_5 (`self.GameHUD`))
  (switch `string` HitResult
    (:`Perfect`
      (set `/Game/BeatShot/UI/GameHUD.Score` (+ 1000 (`/Game/BeatShot/UI/GameHUD.Score` _gamehud_3)) _gamehud_3))
    (:`Great`
      (set `/Game/BeatShot/UI/GameHUD.Score` (+ 750 (`/Game/BeatShot/UI/GameHUD.Score` _gamehud_4)) _gamehud_4))
    (:`Good`
      (set `/Game/BeatShot/UI/GameHUD.Score` (+ 500 (`/Game/BeatShot/UI/GameHUD.Score` _gamehud_2)) _gamehud_2))
    (:`Bad`
      (set `/Game/BeatShot/UI/GameHUD.Score` (+ 200 (`/Game/BeatShot/UI/GameHUD.Score` _gamehud_5)) _gamehud_5))
    (:`Miss`
      (set `/Game/BeatShot/UI/GameHUD.Score` (+ 0 (`/Game/BeatShot/UI/GameHUD.Score` _gamehud)) _gamehud))))

(fn `UserConstructionScript`)